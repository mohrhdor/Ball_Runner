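; BP_cylinder_01 is a crystal-style pickup actor that is drawn into the player and disappears when collected.
; Overlap of Trigger_02 by the first player's pawn plays the Crystaltransform timeline, then destroys the actor when it finishes.
; Each timeline update lerps from current values toward the player's location, zero scale and zero PointLight intensity.
; A 2D sound spawn and a delay are left unconnected, so they never run.
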(event `self.Trigger_02.OnComponentBeginOverlap`
  (params (OverlappedComponent :type "PrimitiveComponent Object Reference") (OtherActor :type "Actor Object Reference") (OtherComp :type "PrimitiveComponent Object Reference") (OtherBodyIndex :type Integer) (bFromSweep :type Boolean) (SweepResult :type "HitResult Structure (by ref)"))
  (bind _pointlight (`self.PointLight`))
  (if (== OtherActor (`GameplayStatics.GetPlayerPawn` 0))
    (bind (_direction _newtrack_0 _crystal_scale _light_intensity) (`Timeline|crystaltransform`)
      (:`Update`
        (`self.K2_SetActorLocation` (`KismetMathLibrary.VLerp` (`self.K2_GetActorLocation`) (`self.K2_GetActorLocation` (`GameplayStatics.GetPlayerPawn` 0)) _newtrack_0))
        (`self.SetActorScale3D` (`KismetMathLibrary.VLerp` (`self.GetActorScale3D`) (0.0 0.0 0.0) _crystal_scale))
        (`LightComponent.SetIntensity` _pointlight (`KismetMathLibrary.Lerp` (`LightComponentBase.Intensity` _pointlight) 0.0 _light_intensity)))
      (:`Finished`
        (`self.K2_DestroyActor`)))))

(fn `UserConstructionScript`)